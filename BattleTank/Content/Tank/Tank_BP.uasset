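; Tank Blueprint that handles the player's aim input for mouse or keyboard and gamepad axes.
; Horizontal input yaws the HorizonGimbal and elevation input pitches the SpringArm, splitting orbit-style aiming across two components.
; Axis values apply directly as local rotation deltas without delta-time scaling, and gamepad elevation is inverted.
; The event graph and construction script contain no active logic.
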(event EventBeginPlay)

(event Collision|EventActorBeginOverlap
  (params (OtherActor :type Actor%20Object%20Reference)))

(event EventTick
  (params (DeltaSeconds :type Float%20%28single-precision%29)))

(event Input|AxisEvents|InputAxisAimHorizon
  (params (AxisValue :type Float%20%28single-precision%29))
  ;[1 1 1] Inputs
  ;;[1 1 1] AimHorizon
  (Transformation|AddLocalRotation (Variables|Default|GetHorizon%20Gimbal) (Math|Rotator|MakeRotator 0.0 0.0 AxisValue) false false))

(event Input|AxisEvents|InputAxisAimElevation
  (params (AxisValue :type Float%20%28single-precision%29))
  ;[1 1 1] Inputs
  ;;[1 1 1] AimElevation
  (Transformation|AddLocalRotation (Variables|Default|GetSpringArm) (Math|Rotator|MakeRotator 0.0 AxisValue 0.0) false false))

(event Input|AxisEvents|InputAxisGamepad_AimHorizon
  (params (AxisValue :type Float%20%28single-precision%29))
  ;[1 1 1] Inputs
  ;;[1 1 1] Gamepad - Horizon
  (Transformation|AddLocalRotation (Variables|Default|GetHorizon%20Gimbal) (Math|Rotator|MakeRotator 0.0 0.0 AxisValue) false false))

(event Input|AxisEvents|InputAxisGamepad_AimElevation
  (params (AxisValue :type Float%20%28single-precision%29))
  ;[1 1 1] Inputs
  ;;[1 1 1] Gamepad - Elevation
  (Transformation|AddLocalRotation (Variables|Default|GetSpringArm) (Math|Rotator|MakeRotator 0.0 (* AxisValue -1.0) 0.0) false false))

(fn ConstructionScript)